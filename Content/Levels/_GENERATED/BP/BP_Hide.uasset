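; Hiding-spot actor with a swinging door that lets the player's HP_Character hide inside and come back out.
; The hiding event passes a gate, plays a timeline rotating the door mesh, and toggles the character's visibility and collision while blending the camera between actor and character.
; Box begin overlap disables input and closes the gate; end overlap stores the character and, like toggling, re-enables both after a short delay or directly.
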(event `hiding`
  (`/Engine/EditorBlueprintResources/StandardMacros.Gate` true :!label _label
    (:`Exit`
      (`|ExecutionSequence`
        (:`then_0`
          (bind (_direction `_새_트랙_0`) (`Timeline|타임라인` :!via `PlayFromStart`)
            (:`Update`
              (`SceneComponent.K2_SetRelativeRotation` (`self.StaticMesh1`) (`KismetMathLibrary.MakeRotator` 0.0 0.0 (`KismetMathLibrary.Lerp` (`self.close`) (`self.open`) `_새_트랙_0`)) false false))))
        (:`then_1`
          (`self.tggle hide`)
          (`KismetSystemLibrary.Delay` 0.2)
          (`self.EnableInput` (`GameplayStatics.GetPlayerController` 0) null :!label _label_2)
          (goto _label :!via `Open`))))))

(event `self.Box.OnComponentEndOverlap`
  (params (OverlappedComponent :type "PrimitiveComponent Object Reference") (OtherActor :type "Actor Object Reference") (OtherComp :type "PrimitiveComponent Object Reference") (OtherBodyIndex :type Integer))
  (bind _ashp_character (cast `/Game/HP_Character` OtherActor))
  (set `self.char REF` _ashp_character)
  (goto _label_2))

(event `self.Box.OnComponentBeginOverlap`
  (params (OverlappedComponent :type "PrimitiveComponent Object Reference") (OtherActor :type "Actor Object Reference") (OtherComp :type "PrimitiveComponent Object Reference") (OtherBodyIndex :type Integer) (bFromSweep :type Boolean) (SweepResult :type "HitResult Structure (by ref)"))
  (cast `/Game/HP_Character` OtherActor)
  (`self.DisableInput` (`GameplayStatics.GetPlayerController` 0))
  (goto _label :!via `Close`))

(fn `tggle hide`
  (bind _returnvalue (`GameplayStatics.GetPlayerController` 0))
  (bind _char_ref (`self.char REF`))
  (if (`self.hiding?`)
    (set `self.hiding?` false)
    (`self.SetActorHiddenInGame` _char_ref false)
    (`self.SetActorEnableCollision` _char_ref true)
    (`PlayerController.SetViewTargetWithBlend` _returnvalue _char_ref 0.6 "VTBlend_Linear" 0.0 false)
    (else
      (set `self.hiding?` true)
      (`self.SetActorHiddenInGame` _char_ref true)
      (`self.SetActorEnableCollision` _char_ref false)
      (`PlayerController.SetViewTargetWithBlend` _returnvalue self 0.6 "VTBlend_Linear" 0.0 false))))

(fn `UserConstructionScript`)