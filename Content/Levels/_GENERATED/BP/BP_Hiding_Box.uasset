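; Hiding-box actor that an HP_Character can use to hide inside.
; Overlapping the box enables input and opens a gate for the hidingbox event; leaving disables both.
; ToggleHide flips character visibility and collision, blending the camera between box and character, though the gated event calls it twice in succession.
; The event also runs Opendoor, where a timeline lerps the door's yaw from closed to open.
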(event `hiding box`
  (`/Engine/EditorBlueprintResources/StandardMacros.Gate` true :!label _label
    (:`Exit`
      (`self.toggle_hide`)
      (`|ExecutionSequence`
        (:`then_0`
          (`self.toggle_hide`)
          (`KismetSystemLibrary.Delay` 0.2)
          (`self.EnableInput` (`GameplayStatics.GetPlayerController` 0) :!label _label_2)
          (goto _label :!via `Open`))
        (:`then_1`
          (bind (_direction _hiding) (`Timeline|hiding` :!via `PlayFromStart`)
            (:`Update`
              (`SceneComponent.K2_SetRelativeRotation` (`self.door`) (`KismetMathLibrary.MakeRotator` 0.0 0.0 (`KismetMathLibrary.Lerp` (`self.close door`) (`self.open door`) _hiding)) false false))))))))

(event `self.Box.OnComponentBeginOverlap`
  (params (OverlappedComponent :type "PrimitiveComponent Object Reference") (OtherActor :type "Actor Object Reference") (OtherComp :type "PrimitiveComponent Object Reference") (OtherBodyIndex :type Integer) (bFromSweep :type Boolean) (SweepResult :type "HitResult Structure (by ref)"))
  (bind _ashp_character (cast `/Game/HP_Character` OtherActor))
  (set `self.As HP Character` _ashp_character)
  (goto _label_2))

(event `self.Box.OnComponentEndOverlap`
  (params (OverlappedComponent :type "PrimitiveComponent Object Reference") (OtherActor :type "Actor Object Reference") (OtherComp :type "PrimitiveComponent Object Reference") (OtherBodyIndex :type Integer))
  (cast `/Game/HP_Character` OtherActor)
  (`self.DisableInput` (`GameplayStatics.GetPlayerController` 0))
  (goto _label :!via `Close`))

(fn `toggle_hide`
  (bind _returnvalue (`GameplayStatics.GetPlayerController` 0))
  (bind _as_hp_character (`self.As HP Character`))
  (if (`self.is hiding`)
    (set `self.is hiding` false)
    (`self.SetActorHiddenInGame` _as_hp_character false)
    (`self.SetActorEnableCollision` _as_hp_character true)
    (`PlayerController.SetViewTargetWithBlend` _returnvalue _as_hp_character 0.6 "VTBlend_Linear" 0.0 false)
    (else
      (set `self.is hiding` true)
      (`self.SetActorHiddenInGame` _as_hp_character true)
      (`self.SetActorEnableCollision` _as_hp_character false)
      (`PlayerController.SetViewTargetWithBlend` _returnvalue self 0.6 "VTBlend_Linear" 0.0 false))))

(fn `UserConstructionScript`)